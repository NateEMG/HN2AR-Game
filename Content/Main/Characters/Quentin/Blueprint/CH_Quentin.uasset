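; Player character Quentin: first-person movement with run, crouch and jump, plus a six-slot item inventory and world interaction.
; Camera line traces drive item pickup, interact messages and a cross/hand crosshair that reacts to "Interactive" components.
; Picked-up items attach to sockets, with only the number-key-selected one visible and usable.
; Releasing Throw/Drop either places the item or, after a hold, throws it with an impulse, while AnimTask tracks each action phase.
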(event Custom|Allow%20Pick%20Up
  (bind _object (Variables|Default|GetObject))
  ;[1 1 1] Pick Up
  (Utilities|FlowControl|Gate false) ; enters at Open
)

(event Custom|Disable%20Pick%20Up
  (bind _object (Variables|Default|GetObject))
  ;[1 1 1] Pick Up
  (Utilities|FlowControl|Gate false) ; enters at Close
)

(event Custom|Hide%20Non%20Selected%20Items
  ;[1 1 1] Tick
  (for (_array_element _array_index) (Variables|Default|GetInventory)
    (Utilities|IsValid _array_element
      (:Is%20Valid
        (Rendering|SetActorHiddenInGame _array_element (not (== _array_index (Variables|Default|GetSelected%20Item))))))))

(event Custom|Manage%20Crosshair
  (bind _inventory_widget (Variables|Default|GetInventory%20Widget))
  (bind (_returnvalue _outhit) (CallFunction|Trace "TraceTypeQuery1" "None" 3e+02))
  (if _returnvalue
    (if (Components|ComponentHasTag (.HitComponent (Collision|BreakHitResult _outhit)) "Interactive")
      (Utilities|FlowControl|Sequence
        (:then_0
          (goto _label_3 Reset))
        (:then_1
          (Utilities|FlowControl|DoOnce false :!label _label
            (:Completed
              (Default|ShowHand _inventory_widget)))))
      (else
        (Utilities|FlowControl|Sequence :!label _label_2
          (:then_0
            (goto _label Reset))
          (:then_1
            (Utilities|FlowControl|DoOnce false :!label _label_3
              (:Completed
                (Default|ShowCross _inventory_widget)))))))
    (else
      (goto _label_2))))

(event EventBeginPlay
  (bind _returnvalue (UserInterface|CreateWidget "/Game/UI/Widget/BPW_Crosshair.BPW_Crosshair_C" (Game|GetPlayerController 0)))
  (UserInterface|Viewport|AddtoViewport _returnvalue 0)
  (Variables|Default|SetInventory%20Widget _returnvalue)
  (bind _returnvalue_2 (UserInterface|CreateWidget "/Game/UI/Widget/BPW_Fade.BPW_Fade_C" (Game|GetPlayerController 0)))
  (UserInterface|Viewport|AddtoViewport _returnvalue_2 0)
  (Default|Fade _returnvalue_2))

(event Collision|EventActorBeginOverlap
  (params (OtherActor :type Actor%20Object%20Reference)))

(event EventTick
  (params (DeltaSeconds :type Float%20%28single-precision%29))
  ;[1 1 1] Tick
  (Utilities|FlowControl|Sequence
    (:then_0
      (bind (_valid _output) (CallFunction|GetHeldObject))
      (if _valid
        (Variables|Default|SetHolding _valid)
        (Variables|Default|SetTwo%20Handed (Variables|/Game/Main/Objects/Blueprint/BP_Base_Item.BP_Base_Item_C|GetTwo%20Handed _output))
        (else
          (Variables|Default|SetHolding _valid))))
    (:then_1
      (CallFunction|HideNonSelectedItems)
      (CallFunction|ManageCrosshair))))

(event Input|ActionEvents|InputActionJump
  (params (Key :type Key%20Structure :default "None"))
  ;[1 1 1] Input
  (:Pressed
    (Character|Jump)))

(event Input|ActionEvents|InputActionRun
  (params (Key :type Key%20Structure :default "None"))
  ;[1 1 1] Input
  (:Pressed
    (CallFunction|SetSpeed (Variables|Default|GetRun%20Speed)))
  (:Released
    (CallFunction|SetSpeed (Variables|Default|GetWalk%20Speed))))

(event Input|ActionEvents|InputActionCrouch
  (params (Key :type Key%20Structure :default "None"))
  ;[1 1 1] Input
  (:Pressed
    (if (AI|Components|NavMovement|IsCrouching (Variables|Character|GetCharacterMovement))
      (Character|UnCrouch)
      (else
        (Character|Crouch)))))

(event Input|ActionEvents|InputActionInteract
  (params (Key :type Key%20Structure :default "None"))
  ;[1 1 1] Interact
  (:Pressed
    (bind (_returnvalue _outhit) (CallFunction|Trace "TraceTypeQuery1" "None" 3e+02))
    (if _returnvalue
      (Class|InteractionInterface|Interact(Message) (.HitActor (Collision|BreakHitResult _outhit)) (.HitComponent (Collision|BreakHitResult _outhit))))))

(event Input|ActionEvents|InputActionThrow/Drop
  (params (Key :type Key%20Structure :default "None"))
  (bind _camera (Variables|Default|GetCamera))
  (bind _object (Variables|Default|GetObject))
  (bind _returnvalue (Transformation|GetWorldRotation _camera))
  (bind _transform_origin (Variables|/Game/Main/Objects/Blueprint/BP_Base_Object.BP_Base_Object_C|GetTransform%20Origin _object))
  ;[1 1 1] Drop / Throw
  (:Pressed
    (Utilities|FlowControl|Gate true) ; enters at Open
  )
  (:Released
    (Utilities|FlowControl|Sequence
      (:then_0
        (Utilities|FlowControl|Gate true) ; enters at Close
      )
      (:then_1
        (Utilities|IsValid (Utilities|Array|Get(acopy) (Variables|Default|GetInventory) (Variables|Default|GetSelected%20Item))
          (:Is%20Valid
            (if (Utilities|Enum|Equal(Enum) (Variables|Default|GetAnim%20Task) "NewEnumerator2")
              (Variables|Default|SetAnim%20Task "NewEnumerator3")
              (Utilities|FlowControl|Delay 0.2)
              (Variables|Default|SetAnim%20Task "NewEnumerator1")
              (bind _location (CallFunction|TraceforDrop "None" 1e+02))
              (bind _item (CallFunction|RemoveSelectedItem (Math|Transform|MakeTransform _location (Math|Rotator|MakeRotator (.roll _returnvalue) (.pitch _returnvalue) (.yaw _returnvalue)) (.scale _transform_origin))))
              (Utilities|FlowControl|Delay 0.05)
              (Default|Drop _item)
              (Physics|AddImpulse (Variables|/Game/Main/Objects/Blueprint/BP_Base_Item.BP_Base_Item_C|GetMesh _item) (* (Math|Rotator|GetRotationXVector (Transformation|GetWorldRotation (Variables|Default|GetCamera))) 5e+04) "None" false)
              (CallFunction|RemovefromInventory)
              (else
                (Variables|Default|SetAnim%20Task "NewEnumerator3")
                (Utilities|FlowControl|Delay 0.2)
                (Variables|Default|SetAnim%20Task "NewEnumerator1")
                (bind _location_2 (CallFunction|TraceforDrop "None" 3e+02))
                (bind _item_2 (CallFunction|RemoveSelectedItem (Math|Transform|MakeTransform _location_2 (Math|Rotator|MakeRotator 0.0 0.0 (.yaw _returnvalue)) (.scale _transform_origin))))
                (Utilities|FlowControl|Delay 0.05)
                (Default|Drop _item_2)
                (CallFunction|RemovefromInventory)))))))))

(event Input|ActionEvents|InputActionUse
  (params (Key :type Key%20Structure :default "None"))
  (bind _selected_item (Variables|Default|GetSelected%20Item))
  (bind _inventory (Variables|Default|GetInventory))
  (bind _output (Utilities|Array|Get(acopy) _inventory _selected_item))
  ;[1 1 1] Use Item
  (:Pressed
    (Utilities|IsValid _output
      (:Is%20Valid
        (Default|Use _output)))))

(event Input|AxisEvents|InputAxisForward
  (params (AxisValue :type Float%20%28single-precision%29))
  ;[1 1 1] Input
  (bind _output_get (Variables|Default|SetForward%20Value AxisValue))
  (Pawn|Input|AddMovementInput (Math|Vector|GetForwardVector (Variables|Collision|GetCapsuleComponent)) _output_get true))

(event Input|AxisEvents|InputAxisRight
  (params (AxisValue :type Float%20%28single-precision%29))
  ;[1 1 1] Input
  (bind _output_get (Variables|Default|SetRight%20Value AxisValue))
  (Pawn|Input|AddMovementInput (Math|Vector|GetRightVector (Variables|Collision|GetCapsuleComponent)) _output_get true))

(event Input|AxisEvents|InputAxisLookUp
  (params (AxisValue :type Float%20%28single-precision%29))
  ;[1 1 1] Input
  (Pawn|Input|AddControllerPitchInput AxisValue))

(event Input|AxisEvents|InputAxisLookRight
  (params (AxisValue :type Float%20%28single-precision%29))
  ;[1 1 1] Input
  (Pawn|Input|AddControllerYawInput AxisValue))

(event Input|AxisEvents|InputAxisThrow
  (params (AxisValue :type Float%20%28single-precision%29))
  ;[1 1 1] Drop / Throw
  (Utilities|IsValid (Utilities|Array|Get(acopy) (Variables|Default|GetInventory) (Variables|Default|GetSelected%20Item))
    (:Is%20Valid
      (Utilities|FlowControl|Gate true
        (:Exit
          (Utilities|IsValid (Utilities|Array|Get(acopy) (Variables|Default|GetInventory) (Variables|Default|GetSelected%20Item))
            (:Is%20Valid
              (if (>= (Class|PlayerController|GetInputKeyTimeDown (Game|GetPlayerController 0) (stale Input|ActionEvents|InputActionThrow/Drop Key)) 0.2)
                (Variables|Default|SetAnim%20Task "NewEnumerator2")))))))))

(event Input|KeyboardEvents|E
  (params (Key :type Key%20Structure :default "None"))
  ;[1 1 1] Pick Up
  (:Pressed
    (if (not (>= (Utilities|Array|Length (Variables|Default|GetInventory)) 6))
      (if (not (and false (not (Utilities|Enum|Equal(Enum) (Variables|Default|GetAnim%20Task) "NewEnumerator1"))))
        (bind (_returnvalue _outhit) (CallFunction|Trace "TraceTypeQuery1" "None" 3e+02))
        (if _returnvalue
          (bind _asbp_base_item (Utilities|Casting|CastToBP_Base_Item (.HitActor (Collision|BreakHitResult _outhit))))
          (bind _output_get (Variables|Default|SetObject _asbp_base_item))
          (if (Variables|/Game/Main/Objects/Blueprint/BP_Base_Item.BP_Base_Item_C|GetCan%20Pick%20Up _output_get)
            (Utilities|FlowControl|Gate false
              (:Exit
                (CallFunction|DisablePickUp)
                (Default|PickUp (Variables|Default|GetObject))
                (Default|RunSocketCreation (Variables|Default|GetObject))
                (bind _returnvalue_2 (Utilities|Array|Add (Variables|Default|GetInventory) (Variables|Default|GetObject)))
                (Variables|Default|SetSelected%20Item _returnvalue_2)
                (Variables|Default|SetAnim%20Task "NewEnumerator0")
                (Utilities|FlowControl|Delay 0.3)
                (Variables|Default|SetAnim%20Task "NewEnumerator1")
                (Transformation|AttachComponentToComponent (Variables|/Game/Main/Objects/Blueprint/BP_Base_Item.BP_Base_Item_C|GetMesh (Variables|Default|GetObject)) (Variables|/Game/Main/Objects/Blueprint/BP_Base_Object.BP_Base_Object_C|GetSocket (Variables|Default|GetObject)) "None" "SnapToTarget" "SnapToTarget" "SnapToTarget" true)
                (Utilities|FlowControl|Delay 0.5)
                (CallFunction|AllowPickUp)))))))))

(event Input|KeyboardEvents|1
  (params (Key :type Key%20Structure :default "None"))
  (:Pressed
    (Utilities|IsValid (Utilities|Array|Get(acopy) (Variables|Default|GetInventory))
      (:Is%20Valid
        (if (not (== (Variables|Default|GetSelected%20Item) 0))
          (Variables|Default|SetSelected%20Item 0))))))

(event Input|KeyboardEvents|2
  (params (Key :type Key%20Structure :default "None"))
  (:Pressed
    (Utilities|IsValid (Utilities|Array|Get(acopy) (Variables|Default|GetInventory) 1)
      (:Is%20Valid
        (if (not (== (Variables|Default|GetSelected%20Item) 1))
          (Variables|Default|SetSelected%20Item 1))))))

(event Input|KeyboardEvents|3
  (params (Key :type Key%20Structure :default "None"))
  (:Pressed
    (Utilities|IsValid (Utilities|Array|Get(acopy) (Variables|Default|GetInventory) 2)
      (:Is%20Valid
        (if (not (== (Variables|Default|GetSelected%20Item) 2))
          (Variables|Default|SetSelected%20Item 2))))))

(event Input|KeyboardEvents|4
  (params (Key :type Key%20Structure :default "None"))
  (:Pressed
    (Utilities|IsValid (Utilities|Array|Get(acopy) (Variables|Default|GetInventory) 3)
      (:Is%20Valid
        (if (not (== (Variables|Default|GetSelected%20Item) 3))
          (Variables|Default|SetSelected%20Item 3))))))

(event Input|KeyboardEvents|5
  (params (Key :type Key%20Structure :default "None"))
  (:Pressed
    (Utilities|IsValid (Utilities|Array|Get(acopy) (Variables|Default|GetInventory) 4)
      (:Is%20Valid
        (if (not (== (Variables|Default|GetSelected%20Item) 4))
          (Variables|Default|SetSelected%20Item 4))))))

(event Input|KeyboardEvents|6
  (params (Key :type Key%20Structure :default "None"))
  (:Pressed
    (Utilities|IsValid (Utilities|Array|Get(acopy) (Variables|Default|GetInventory) 5)
      (:Is%20Valid
        (if (== (Variables|Default|GetSelected%20Item) 5)
          (Variables|Default|SetSelected%20Item 5))))))

(fn ConstructionScript)

(fn SetSpeed
  (params (MaxWalkSpeed :type Float%20%28single-precision%29))
  (Variables|/Script/Engine.CharacterMovementComponent|SetMaxWalkSpeed (Variables|Character|GetCharacterMovement) MaxWalkSpeed))

(fn Trace
  (params (TraceChannel :type ETraceTypeQuery%20Enum :default "TraceTypeQuery1") (DrawDebugType :type EDrawDebugTrace%20Enum :default "None") (Trace%20Length :type Float%20%28single-precision%29))
  (bind _camera (Variables|Default|GetCamera))
  (bind _returnvalue (Transformation|GetWorldLocation _camera))
  (bind (_outhit _returnvalue_2) (Collision|LineTraceByChannel _returnvalue (+ _returnvalue (* (Math|Vector|GetForwardVector _camera) Trace%20Length)) TraceChannel false (Utilities|Array|MakeArray self) DrawDebugType))
  (return _returnvalue_2 _outhit))

(fn GetHeldObject
  (bind _inventory (Variables|Default|GetInventory))
  (bind _selected_item (Variables|Default|GetSelected%20Item))
  (bind _output (Utilities|Array|Get(acopy) _inventory _selected_item))
  (Utilities|IsValid _output
    (:Is%20Valid
      (return true _output))
    (:Is%20Not%20Valid
      (return false 0))))

(fn TraceforDrop
  (params (DrawDebugType :type EDrawDebugTrace%20Enum :default "None") (Trace%20Length :type Float%20%28single-precision%29))
  (bind (_returnvalue _outhit) (CallFunction|Trace "TraceTypeQuery1" DrawDebugType Trace%20Length))
  (if _returnvalue
    (return (.ImpactPoint (Collision|BreakHitResult _outhit)))
    (else
      (return (.TraceEnd (Collision|BreakHitResult _outhit))))))

(fn RemoveSelectedItem
  (params (NewTransform :type Transform%20%28by%20ref%29))
  (bind (_valid _output) (CallFunction|GetHeldObject))
  (if _valid
    (Transformation|DetachFromComponent (Variables|/Game/Main/Objects/Blueprint/BP_Base_Item.BP_Base_Item_C|GetMesh _output) "KeepRelative" "KeepRelative" "KeepRelative" true)
    (Transformation|SetWorldTransform (Variables|/Game/Main/Objects/Blueprint/BP_Base_Item.BP_Base_Item_C|GetMesh _output) NewTransform false false)
    (return _output)))

(fn RemovefromInventory
  (Utilities|Array|RemoveItem (Variables|Default|GetInventory) (Utilities|Array|Get(acopy) (Variables|Default|GetInventory) (Variables|Default|GetSelected%20Item)))
  (if (> (Variables|Default|GetSelected%20Item) 0)
    (Math|Integer|DecrementInt (Variables|Default|GetSelected%20Item)
      (:%20%20
        (return)))
    (else
      (Variables|Default|SetSelected%20Item 0))))